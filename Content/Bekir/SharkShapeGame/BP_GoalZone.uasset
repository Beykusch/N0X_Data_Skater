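; BP_GoalZone is the finish trigger of the shark shape game that ends the run with a win.
; Any overlap with GoalBox stops BP_Shark chasing, as the flag is cleared before the player cast.
; For BP_SharkShape_Player, it prints a win message and disables movement.
; It then shows WBP_DeathScreen, reused for the win, with mouse cursor and UI-only input.
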(event OnComponentBeginOverlap(GoalBox)
  (params (OverlappedComponent :type Primitive%20Component%20Object%20Reference) (OtherActor :type Actor%20Object%20Reference) (OtherComp :type Primitive%20Component%20Object%20Reference) (OtherBodyIndex :type Integer) (bFromSweep :type Boolean) (SweepResult :type Hit%20Result%20Structure%20%28by%20ref%29))
  (bind _returnvalue (Game|GetPlayerController 0))
  (bind _returnvalue_2 (Actor|GetActorOfClass "/Game/Mert/Shark_Mode/BP_Shark.BP_Shark_C"))
  (Variables|/Game/Mert/Shark_Mode/BP_Shark.BP_Shark_C|SetisChasing _returnvalue_2 false)
  (bind _asbp_shark_shape_player (Utilities|Casting|CastToBP_SharkShape_Player OtherActor))
  (if true
    (Development|PrintString "YOU WIN")
    (bind _ascharacter (Utilities|Casting|CastToCharacter _asbp_shark_shape_player))
    (Pawn|Components|CharacterMovement|DisableMovement (Variables|/Script/Engine.Character|GetCharacterMovement _ascharacter))
    (bind _returnvalue_3 (UserInterface|CreateWidget "/Game/Bekir/UI/WBP_DeathScreen.WBP_DeathScreen_C" _returnvalue))
    (UserInterface|Viewport|AddtoViewport _returnvalue_3 0)
    (Variables|/Script/Engine.PlayerController|SetbShowMouseCursor _returnvalue true)
    (Input|SetInputModeUIOnly _returnvalue _returnvalue_3 "DoNotLock" false)))

(event EventBeginPlay)

(event Collision|EventActorBeginOverlap
  (params (OtherActor :type Actor%20Object%20Reference)))

(event EventTick
  (params (DeltaSeconds :type Float%20%28single-precision%29)))

(fn ConstructionScript)