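; D12 platform actor that rolls about one of five horizontal axes, spaced like pentagon edges, via the W, E, D, A and Q keys.
; StartRoll ignores input while rolling, picks the axis and computes a target from FlatRotation plus RollAngle.
; A roll timeline applies incremental world-space rotation from alpha deltas.
; A settle timeline then lerps along the shortest path to the exact target, snaps and unlocks input.
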(event Custom|StartRoll
  (params (Direction :type Integer))
  (if (not (Variables|Default|GetIsRolling))
    (Variables|Default|SetIsRolling true)
    (Variables|Default|SetStartRotation (Transformation|GetActorRotation))
    (Variables|Default|SetLastAlpha 0.0)
    (switch int Direction
      (:0
        (bind _output_get (Variables|Default|SetRollAxis (Math|Vector|MakeVector 0.0 1.0 0.0)))
        (Variables|Default|SetTargetRotation (Math|Rotator|CombineRotators (Variables|Default|GetFlatRotation) (Math|Vector|RotatorfromAxisandAngle _output_get (Variables|Default|GetRollAngle))))
        (bind _alpha (Timeline|TL_Roll2 PlayFromStart)
          (:Update
            (Class|Actor|AddActorWorldRotation (Math|Vector|RotatorfromAxisandAngle (Variables|Default|GetRollAxis) (* (- _alpha (Variables|Default|GetLastAlpha)) (Variables|Default|GetRollAngle))))
            (Variables|Default|SetLastAlpha _alpha))
          (:Finished
            (bind _output_get_2 (Variables|Default|SetCorrectionStartRotation (Transformation|GetActorRotation)))
            (bind _alpha_2 (Timeline|TL_Settle PlayFromStart)
              (:Update
                (Transformation|SetActorRotation (Math|Rotator|Lerp(Rotator) _output_get_2 (Variables|Default|GetTargetRotation) _alpha_2 true)))
              (:Finished
                (Transformation|SetActorRotation (Variables|Default|GetTargetRotation))
                (Variables|Default|SetIsRolling false))))))
      (:1
        (bind _output_get_3 (Variables|Default|SetRollAxis (Math|Vector|MakeVector -0.951 0.309 0.0)))
        (Variables|Default|SetTargetRotation (Math|Rotator|CombineRotators (Variables|Default|GetFlatRotation) (Math|Vector|RotatorfromAxisandAngle _output_get_3 (Variables|Default|GetRollAngle))))
        (Timeline|TL_Roll2 PlayFromStart))
      (:2
        (bind _output_get_4 (Variables|Default|SetRollAxis (Math|Vector|MakeVector -0.588 -0.809 0.0)))
        (Variables|Default|SetTargetRotation (Math|Rotator|CombineRotators (Variables|Default|GetFlatRotation) (Math|Vector|RotatorfromAxisandAngle _output_get_4 (Variables|Default|GetRollAngle))))
        (Timeline|TL_Roll2 PlayFromStart))
      (:3
        (bind _output_get_5 (Variables|Default|SetRollAxis (Math|Vector|MakeVector 0.588 -0.809 0.0)))
        (Variables|Default|SetTargetRotation (Math|Rotator|CombineRotators (Variables|Default|GetFlatRotation) (Math|Vector|RotatorfromAxisandAngle _output_get_5 (Variables|Default|GetRollAngle))))
        (Timeline|TL_Roll2 PlayFromStart))
      (:4
        (bind _output_get_6 (Variables|Default|SetRollAxis (Math|Vector|MakeVector 0.951 0.309 0.0)))
        (Variables|Default|SetTargetRotation (Math|Rotator|CombineRotators (Variables|Default|GetFlatRotation) (Math|Vector|RotatorfromAxisandAngle _output_get_6 (Variables|Default|GetRollAngle))))
        (Timeline|TL_Roll2 PlayFromStart)))))

(event Collision|EventActorBeginOverlap
  (params (OtherActor :type Actor%20Object%20Reference)))

(event EventTick
  (params (DeltaSeconds :type Float%20%28single-precision%29)))

(event Input|KeyboardEvents|Q
  (params (Key :type Key%20Structure :default "None"))
  (:Pressed
    (CallFunction|StartRoll 4)))

(event Input|KeyboardEvents|W
  (params (Key :type Key%20Structure :default "None"))
  (:Pressed
    (CallFunction|StartRoll)))

(event Input|KeyboardEvents|E
  (params (Key :type Key%20Structure :default "None"))
  (:Pressed
    (CallFunction|StartRoll 1)))

(event Input|KeyboardEvents|A
  (params (Key :type Key%20Structure :default "None"))
  (:Pressed
    (CallFunction|StartRoll 3)))

(event Input|KeyboardEvents|D
  (params (Key :type Key%20Structure :default "None"))
  (:Pressed
    (CallFunction|StartRoll 2)))

(fn ConstructionScript)