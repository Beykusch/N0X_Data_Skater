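; BP_WorldCube is a cube actor that turns in four directions, using two separate rotation mechanisms.
; Rotate steps the Cube component one degree per looping timer tick for 90 steps, with a flag blocking new turns until it finishes.
; Right, Left, Up and Down compose new values into TargetRotation through CombineRotators.
; Tick continuously eases the whole actor toward that target with RInterpTo.
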(event Custom|Left
  (Variables|Default|SetTargetRotation (Math|Rotator|CombineRotators (Variables|Default|GetTargetRotation) (Math|Rotator|MakeRotator (- (.roll (Variables|Default|GetTargetRotation)) 9e+01) (.pitch (Variables|Default|GetTargetRotation)) (.yaw (Variables|Default|GetTargetRotation))))))

(event Custom|Right
  (Variables|Default|SetTargetRotation (Math|Rotator|CombineRotators (Variables|Default|GetTargetRotation) (Math|Rotator|MakeRotator (+ (.roll (Variables|Default|GetTargetRotation)) 9e+01) (.pitch (Variables|Default|GetTargetRotation)) (.yaw (Variables|Default|GetTargetRotation))))))

(event Custom|Rotate
  (params (Way :type Ways%20Enum :default "NewEnumerator0"))
  (if (Variables|Default|GetBool)
    (Variables|Default|SetBool false)
    (Variables|Default|SetWay Way)
    (Variables|Default|Set31 0)
    (bind _returnvalue (Utilities|Time|SetTimerbyEvent (delegate Custom|2) 0.005 true))))

(event Custom|Down
  (Variables|Default|SetTargetRotation (Math|Rotator|CombineRotators (Variables|Default|GetTargetRotation) (Math|Rotator|MakeRotator (.roll (Variables|Default|GetTargetRotation)) -9e+01 (.yaw (Variables|Default|GetTargetRotation))))))

(event Custom|Up
  (Variables|Default|SetTargetRotation (Math|Rotator|CombineRotators (Variables|Default|GetTargetRotation) (Math|Rotator|MakeRotator (.roll (Variables|Default|GetTargetRotation)) 9e+01 (.yaw (Variables|Default|GetTargetRotation))))))

(event Custom|2
  (Transformation|AddWorldRotation (Variables|Default|GetCube) (Utilities|Select :Index (Variables|Default|GetWay) :NewEnumerator0 "-1.000000,0.000000,0.000000" :NewEnumerator1 "1.000000,0.000000,0.000000" :NewEnumerator2 "0.000000,0.000000,1.000000" :NewEnumerator3 "0.000000,0.000000,-1.000000") false false)
  (bind _result (Math|Integer|IncrementInt (Variables|Default|Get31))
    (:%20%20
      (if (>= _result 90)
        (Utilities|Time|ClearandInvalidateTimerbyHandle (stale Custom|Rotate _returnvalue))
        (Variables|Default|SetBool true)))))

(event EventTick
  (params (DeltaSeconds :type Float%20%28single-precision%29))
  (Transformation|SetActorRotation (Math|Interpolation|RInterpTo (Transformation|GetActorRotation) (Variables|Default|GetTargetRotation) DeltaSeconds 1e+01)))

(fn ConstructionScript)