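; Life_Cube is an actor Blueprint that periodically tumbles its Cube component in random quarter-turn steps.
; A looping three-second timer combines the current world rotation with a randomly chosen axis and direction to set a target.
; A fast secondary timer eases toward it with RInterpTo and is cleared after half a second.
; A Timeline-based Rotate event and disconnected rotation nodes also remain, with no caller in this graph.
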(event Custom|Rotate
  (bind _returnvalue (Math|Random|RandomBool))
  (bind _cube (Variables|Default|GetCube))
  (bind _cube_2 (Variables|Default|GetCube))
  (bind _returnvalue_2 (Transformation|GetWorldRotation _cube))
  (bind _returnvalue_3 (Transformation|GetWorldRotation _cube_2))
  (bind _returnvalue_4 (select _returnvalue -1.0 1.0))
  (bind _returnvalue_5 (* 9e+01 _returnvalue_4))
  (Variables|Default|SetStartRotation (Transformation|GetWorldRotation (Variables|Default|GetCube)))
  (Variables|Default|SetTargetRotation (Utilities|Select :Index (Math|Random|RandomIntegerinRange 0 1) :Option%200 (Math|Rotator|MakeRotator (+ (.roll _returnvalue_3) _returnvalue_5) (.pitch _returnvalue_3) (.yaw _returnvalue_3)) :Option%201 (Math|Rotator|MakeRotator (.roll _returnvalue_2) (+ (.pitch _returnvalue_2) _returnvalue_5) (.yaw _returnvalue_2))))
  (Variables|Default|SetRandomRot (Math|Random|RandomBool))
  (bind _cube_3 (Timeline|RotationTimeline PlayFromStart)
    (:Update
      (Transformation|AddWorldRotation (Variables|Default|GetCube) (select (Variables|Default|GetRandomRot) "3.000000,0.000000,0.000000" "0.000000,0.000000,3.000000") false false))))

(event Custom|Rotator
  (Variables|Default|SetTargetRotation (Math|Rotator|CombineRotators (Transformation|GetWorldRotation (Variables|Default|GetCube)) (* (Utilities|Select :Index (Math|Random|RandomIntegerinRange 0 1) :Option%200 "0.000000,0.000000,90.000000" :Option%201 "-90.000000,0.000000,0.000000") (select (Variables|Default|GetRandomDirection) -1.0 1.0))))
  (Utilities|FlowControl|Sequence
    (:then_0
      (Variables|Default|SetRandomRot (Math|Random|RandomBool))
      (Variables|Default|SetRandomDirection (Math|Random|RandomBool))
      (bind _returnvalue (Utilities|Time|SetTimerbyEvent (delegate Custom|RotatorTimer) 0.01 true))
      (Variables|Default|SetTimerHandler _returnvalue))
    (:then_1
      (Utilities|FlowControl|Delay 0.5)
      (Utilities|Time|ClearandInvalidateTimerbyHandle (Variables|Default|GetTimerHandler)))))

(event Custom|RotatorTimer
  (Transformation|SetWorldRotation (Variables|Default|GetCube) (Math|Interpolation|RInterpTo (Transformation|GetWorldRotation (Variables|Default|GetCube)) (Variables|Default|GetTargetRotation) (Utilities|Time|GetWorldDeltaSeconds) 5.0) false false))

(event EventBeginPlay
  (Utilities|Time|SetTimerbyEvent (delegate Custom|Rotator) 3.0 true))

(fn ConstructionScript)