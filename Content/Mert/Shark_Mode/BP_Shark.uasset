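; Shark hazard for Shark Mode that follows the player and leaps up from below to bite.
; Tick eases its X/Y toward the player with VInterpTo until horizontally close, then stops chasing and starts the attack.
; Chained timelines scale an AttackMark warning, then animate the shark's jump with the bite collision raised, before resetting and resuming the chase after a short delay.
; Bite overlaps kill any unshielded BP_SharkShape_Player.
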(event OnComponentBeginOverlap(Bite_Collision)
  (params (OverlappedComponent :type Primitive%20Component%20Object%20Reference) (OtherActor :type Actor%20Object%20Reference) (OtherComp :type Primitive%20Component%20Object%20Reference) (OtherBodyIndex :type Integer) (bFromSweep :type Boolean) (SweepResult :type Hit%20Result%20Structure%20%28by%20ref%29))
  (bind _asbp_shark_shape_player (Utilities|Casting|CastToBP_SharkShape_Player OtherActor))
  (if (not (Variables|/Game/Bekir/SharkShapeGame/BP_SharkShape_Player.BP_SharkShape_Player_C|GetIsShielded _asbp_shark_shape_player))
    (Default|Die _asbp_shark_shape_player)))

(event Custom|StartSharkAttack
  (Rendering|SetVisibility (Variables|Default|GetCylinder) false false)
  (bind _decal (Timeline|Shark_Indicator PlayFromStart)
    (:Update
      (Transformation|SetRelativeScale3D (Variables|Default|GetAttackMark) (Math|Conversions|ToVector(Float) _decal)))
    (:Finished
      (Transformation|SetRelativeScale3D (Variables|Default|GetAttackMark) "0, 0, 0")
      (Transformation|SetRelativeLocation (Variables|Default|GetBite_Collision) "0.000000,0.000000,-30.000000" false false)
      (bind _zıplama (Timeline|Shark_Jump PlayFromStart)
        (:Update
          (Transformation|SetRelativeLocation (Variables|Default|GetShark) (Math|Vector|Lerp(Vector) "0.000000,0.000000,-790.000000" "0.000000,0.000000,-70.000000" _zıplama) false false))
        (:Finished
          (Transformation|SetRelativeLocation (Variables|Default|GetShark) "0.000000,0.000000,-790.000000" false false)
          (Transformation|SetRelativeLocation (Variables|Default|GetBite_Collision) "0.000000,0.000000,-140.000000" false false)
          (Utilities|FlowControl|Delay 0.5)
          (Development|PrintString "Hello" true true "(R=0.000000,G=1.000000,B=0.020574,A=1.000000)")
          (Rendering|SetVisibility (Variables|Default|GetCylinder) true false)
          (Variables|Default|SetisChasing true))))))

(event Custom|StartChase)

(event EventTick
  (params (DeltaSeconds :type Float%20%28single-precision%29))
  (bind _returnvalue (Game|GetPlayerCharacter 0))
  (bind _returnvalue_2 (Transformation|GetActorLocation))
  (bind _returnvalue_3 (Transformation|GetActorLocation _returnvalue))
  (bind _returnvalue_4 (Math|Interpolation|VInterpTo _returnvalue_2 _returnvalue_3 DeltaSeconds 1.5))
  (if (Variables|Default|GetisChasing)
    (Transformation|SetActorLocation (Math|Vector|MakeVector (.x _returnvalue_4) (.y _returnvalue_4) 0.0) false false)
    (if (and (< (Transformation|GetHorizontalDistanceTo (Game|GetPlayerCharacter 0) self) 7e+01) (Variables|Default|GetisChasing))
      (Variables|Default|SetisChasing false)
      (CallFunction|StartSharkAttack))))

(event EventBeginPlay
  (Variables|Default|SetisChasing true))

(fn ConstructionScript)