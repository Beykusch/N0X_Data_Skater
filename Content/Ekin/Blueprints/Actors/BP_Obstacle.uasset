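; Moving obstacle that tests whether BP_Ekinigga is jumping or diving when it hits it.
; The construction script shows the base or high mesh according to ObstacleType (Jump or Dive).
; Tick moves it along world Z by Speed and destroys it above a height limit.
; Both meshes share one overlap check that adds or resets the player's bonus, then destroys the obstacle.
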(event OnComponentBeginOverlap(SM_Base)
  (params (OverlappedComponent :type Primitive%20Component%20Object%20Reference) (OtherActor :type Actor%20Object%20Reference) (OtherComp :type Primitive%20Component%20Object%20Reference) (OtherBodyIndex :type Integer) (bFromSweep :type Boolean) (SweepResult :type Hit%20Result%20Structure%20%28by%20ref%29))
  (bind _obstacletype (Variables|Default|GetObstacleType))
  (Utilities|Casting|CastToBP_Ekinigga OtherActor)
  (bind _asbp_ekinigga (Utilities|Casting|CastToBP_Ekinigga (stale OnComponentBeginOverlap(SM_High) OtherActor)))
  (if (== _obstacletype "Jump")
    (if (Variables|/Game/Ekin/Blueprints/Core/BP_Ekinigga.BP_Ekinigga_C|GetIsJumping _asbp_ekinigga)
      (Default|AddBonus _asbp_ekinigga :!label _label)
      (else
        (Default|ResetBonus _asbp_ekinigga :!label _label_2)))
    (Actor|DestroyActor)
    (elif (== _obstacletype "Dive")
      (if (Variables|/Game/Ekin/Blueprints/Core/BP_Ekinigga.BP_Ekinigga_C|GetIsDiving _asbp_ekinigga)
        (goto _label)
        (else
          (goto _label_2))))))

(event OnComponentBeginOverlap(SM_High)
  (params (OverlappedComponent :type Primitive%20Component%20Object%20Reference) (OtherActor :type Actor%20Object%20Reference) (OtherComp :type Primitive%20Component%20Object%20Reference) (OtherBodyIndex :type Integer) (bFromSweep :type Boolean) (SweepResult :type Hit%20Result%20Structure%20%28by%20ref%29))
  (bind _obstacletype (Variables|Default|GetObstacleType))
  (Utilities|Casting|CastToBP_Ekinigga (stale OnComponentBeginOverlap(SM_Base) OtherActor))
  (bind _asbp_ekinigga (Utilities|Casting|CastToBP_Ekinigga OtherActor))
  (if (== _obstacletype "Jump")
    (if (Variables|/Game/Ekin/Blueprints/Core/BP_Ekinigga.BP_Ekinigga_C|GetIsJumping _asbp_ekinigga)
      (Default|AddBonus _asbp_ekinigga :!label _label)
      (else
        (Default|ResetBonus _asbp_ekinigga :!label _label_2)))
    (Actor|DestroyActor)
    (elif (== _obstacletype "Dive")
      (if (Variables|/Game/Ekin/Blueprints/Core/BP_Ekinigga.BP_Ekinigga_C|GetIsDiving _asbp_ekinigga)
        (goto _label)
        (else
          (goto _label_2))))))

(event EventBeginPlay)

(event Collision|EventActorBeginOverlap
  (params (OtherActor :type Actor%20Object%20Reference)))

(event EventTick
  (params (DeltaSeconds :type Float%20%28single-precision%29))
  (Transformation|AddActorWorldOffset (Math|Vector|MakeVector 0.0 0.0 (* (Utilities|Time|GetWorldDeltaSeconds) (Variables|Default|GetSpeed))))
  (if (> (.Z (Math|Vector|BreakVector (Transformation|GetActorLocation))) 1e+03)
    (Actor|DestroyActor)))

(fn ConstructionScript
  (bind _sm_base (Variables|Default|GetSM_Base))
  (bind _sm_high (Variables|Default|GetSM_High))
  (switch name (Variables|Default|GetObstacleType)
    (:Jump
      (Rendering|SetVisibility _sm_base true false)
      (Rendering|SetVisibility _sm_high false false))
    (:Dive
      (Rendering|SetVisibility _sm_high true false)
      (Rendering|SetVisibility _sm_base false false))))