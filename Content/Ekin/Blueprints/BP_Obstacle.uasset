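; BP_Obstacle is an obstacle that tests whether the character overlapping it is jumping or diving, as its type requires.
; Tick moves it along world Z at Speed and destroys it once it rises above a fixed height.
; Box overlap casts to the character and compares ObstacleType with its jump or dive flag.
; For either type it only prints success or hit, then destroys itself.
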(event OnComponentBeginOverlap(Box)
  (params (OverlappedComponent :type Primitive%20Component%20Object%20Reference) (OtherActor :type Actor%20Object%20Reference) (OtherComp :type Primitive%20Component%20Object%20Reference) (OtherBodyIndex :type Integer) (bFromSweep :type Boolean) (SweepResult :type Hit%20Result%20Structure%20%28by%20ref%29))
  (bind _obstacletype (Variables|Default|GetObstacleType))
  (bind _asbp_ekinigga (Utilities|Casting|CastToBP_Ekinigga OtherActor))
  (if (== _obstacletype "Jump")
    (if (Variables|/Game/Ekin/Blueprints/BP_Ekinigga.BP_Ekinigga_C|GetIsJumping _asbp_ekinigga)
      (Development|PrintString "SUCCESS! Jumped" true true "(R=0.000000,G=1.000000,B=0.000000,A=1.000000)")
      (else
        (Development|PrintString "HIT! didnt jumped" true true "(R=1.000000,G=0.000000,B=0.000000,A=1.000000)")))
    (Actor|DestroyActor :!label _label)
    (elif (== _obstacletype "Dive")
      (if (Variables|/Game/Ekin/Blueprints/BP_Ekinigga.BP_Ekinigga_C|GetIsDiving _asbp_ekinigga)
        (Development|PrintString "SUCCESS! you dived" true true "(R=0.000000,G=1.000000,B=0.000000,A=1.000000)")
        (goto _label)
        (else
          (Development|PrintString "HIT! you didnt dived" true true "(R=1.000000,G=0.000000,B=0.000000,A=1.000000)")
          (goto _label))))))

(event EventBeginPlay)

(event Collision|EventActorBeginOverlap
  (params (OtherActor :type Actor%20Object%20Reference)))

(event EventTick
  (params (DeltaSeconds :type Float%20%28single-precision%29))
  (Transformation|AddActorWorldOffset (Math|Vector|MakeVector 0.0 0.0 (* (Utilities|Time|GetWorldDeltaSeconds) (Variables|Default|GetSpeed))))
  (if (> (.Z (Math|Vector|BreakVector (Transformation|GetActorLocation))) 1e+03)
    (Actor|DestroyActor)))

(fn ConstructionScript)